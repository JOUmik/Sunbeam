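; BP_Repair is an actor that shows a destroyed object repairing itself through a Geometry Cache animation when P is pressed.
; The first press hides Destruction2, reveals the cache, plays it backwards from the end and starts a Timeline that pauses it on finish.
; A Switch flag sends later presses through paired FlipFlops that alternate cache playback between forward and reverse, alongside the Timeline.
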(event EventBeginPlay
  (Input|EnableInput (Game|GetPlayerController 0)))

(event Input|KeyboardEvents|P
  (params (Key :type Key%20Structure :default "None"))
  (bind _geometrycache (Variables|Default|GetGeometryCache))
  (bind _geometrycache_2 (Variables|Default|GetGeometryCache))
  (:Pressed
    (Utilities|FlowControl|Sequence
      (:then_0
        (Rendering|SetVisibility _geometrycache true false)
        (if (not (Variables|Default|GetSwitch))
          (Class|GeometryCacheComponent|PlayReversedfromEnd _geometrycache)
          (Timeline|Timeline Play
            (:Finished
              (Sequencer|Player|Pause _geometrycache_2)))
          (else
            (Utilities|FlowControl|Sequence
              (:then_0
                (Utilities|FlowControl|FlipFlop
                  (:A
                    (Audio|Components|Audio|Play _geometrycache_2))
                  (:B
                    (Class|GeometryCacheComponent|PlayReversed _geometrycache_2))))
              (:then_1
                (Utilities|FlowControl|FlipFlop
                  (:A
                    (Timeline|Timeline Play))
                  (:B
                    (Timeline|Timeline Reverse))))))))
      (:then_1
        (if (not (Variables|Default|GetSwitch))
          (Variables|Default|SetSwitch true)
          (Rendering|SetVisibility (Variables|Default|Getdestruction2) false false))))))

(fn ConstructionScript)