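; Test actor that line traces along the directional light's axis and changes its cube's material based on the result.
; Each tick it finds the first DirectionalLight and traces from its own location along that light's forward vector, scaled by TraceLength and LengthUnit, against WorldStatic objects.
; A hit or miss selects between two materials on the Cube.
; It also draws the trace and prints the hit actor's name every frame for debugging.
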(event EventBeginPlay)

(event Collision|EventActorBeginOverlap
  (params (OtherActor :type Actor%20Object%20Reference)))

(event EventTick
  (params (DeltaSeconds :type Float%20%28single-precision%29))
  (bind _returnvalue (Transformation|GetActorLocation))
  (bind _outactors (Actor|GetAllActorsOfClass "/Script/Engine.DirectionalLight"))
  (bind (_outhit _returnvalue_2) (Collision|LineTraceForObjects _returnvalue (+ _returnvalue (* (* (Math|Vector|GetForwardVector (Transformation|GetActorRotation (Utilities|Array|Get(acopy) _outactors))) (Variables|Default|GetTraceLength)) (Variables|Default|GetLengthUnit))) (Utilities|Array|MakeArray "ObjectTypeQuery1") false 0 "ForOneFrame"))
  (if _returnvalue_2
    (Rendering|Material|SetMaterial (Variables|Default|GetCube) 0 "/Engine/MapTemplates/Materials/BasicAsset01.BasicAsset01")
    (else
      (Rendering|Material|SetMaterial (Variables|Default|GetCube) 0 "/Game/LevelPrototyping/Materials/MI_Solid_Blue.MI_Solid_Blue")))
  (Development|PrintString (Utilities|GetDisplayName (.HitActor (Collision|BreakHitResult _outhit)))))

(fn ConstructionScript)