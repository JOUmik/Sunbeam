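; BP_Music is a music controller that lets the player toggle FMOD audio parameters from the keyboard, apparently to switch music tracks.
; It enables player input on BeginPlay and listens to number keys 1 through 4.
; Each key drives its own FlipFlop, stores the toggle state and sends it as a number to the FMOD audio component.
; Only key 2 explicitly names its parameter, Track_2.
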(event EventBeginPlay
  (Input|EnableInput (Game|GetPlayerController 0)))

(event Input|KeyboardEvents|4
  (params (Key :type Key%20Structure :default "None"))
  (:Pressed
    (bind _isa (Utilities|FlowControl|FlipFlop)
      (:A
        _)
      (:B
        _))
    (bind _output_get (Variables|Default|SetValue4 _isa))
    (Class|FMODAudioComponent|SetParameter (Variables|Default|GetFMODAudio) "Track_4" (Math|Conversions|ToFloat(Boolean) _output_get))))

(event Input|KeyboardEvents|1
  (params (Key :type Key%20Structure :default "None"))
  (:Pressed
    (bind _isa (Utilities|FlowControl|FlipFlop)
      (:A
        _)
      (:B
        _))
    (bind _output_get (Variables|Default|SetValue1 _isa))
    (Class|FMODAudioComponent|SetParameter (Variables|Default|GetFMODAudio) "Track_1" (Math|Conversions|ToFloat(Boolean) _output_get))))

(event Input|KeyboardEvents|2
  (params (Key :type Key%20Structure :default "None"))
  (:Pressed
    (bind _isa (Utilities|FlowControl|FlipFlop)
      (:A
        _)
      (:B
        _))
    (bind _output_get (Variables|Default|SetValue2 _isa))
    (Class|FMODAudioComponent|SetParameter (Variables|Default|GetFMODAudio) "Track_2" (Math|Conversions|ToFloat(Boolean) _output_get))))

(event Input|KeyboardEvents|3
  (params (Key :type Key%20Structure :default "None"))
  (:Pressed
    (bind _isa (Utilities|FlowControl|FlipFlop)
      (:A
        _)
      (:B
        _))
    (bind _output_get (Variables|Default|SetValue3 _isa))
    (Class|FMODAudioComponent|SetParameter (Variables|Default|GetFMODAudio) "Track_3" (Math|Conversions|ToFloat(Boolean) _output_get))))

(fn ConstructionScript)