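; BP_ControlPawn is a control pawn for a light-beam scene that can take input from serial hardware.
; Its ChangeMirror and ChangeLightBeam events find BP_Beam to set its focal model and sunbeam color.
; When UseHardware is set, BPReadDate reads the serial-com actor and passes its light, map and button indices to change-handlers for light, map and mirror, which are defined outside these graphs.
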(event EventBeginPlay)

(event Collision|EventActorBeginOverlap
  (params (OtherActor :type Actor%20Object%20Reference)))

(event EventTick
  (params (DeltaSeconds :type Float%20%28single-precision%29)))

(event EventChangeMirror
  (params (bShow :type Boolean))
  (bind _returnvalue (Actor|GetActorOfClass "/Game/Blueprints/BP_Beam.BP_Beam_C"))
  (Utilities|IsValid _returnvalue
    (:Is%20Valid
      (Default|SetFocalModel _returnvalue bShow))))

(event EventChangeLightBeam
  (bind _returnvalue (Actor|GetActorOfClass "/Game/Blueprints/BP_Beam.BP_Beam_C"))
  (Utilities|IsValid _returnvalue
    (:Is%20Valid
      (Default|SetSunbeamColor _returnvalue))))

(fn ConstructionScript)

(fn BPReadDate
  (if (Variables|Default|GetUseHardware)
    (bind _returnvalue (Actor|GetActorOfClass "/Game/Blueprints/BP_SerialCom_v4_UE510.BP_SerialCom_v4_UE510_C"))
    (Utilities|IsValid _returnvalue
      (:Is%20Valid
        (Variables|Default|SetSerial%20Com _returnvalue)
        (Utilities|FlowControl|Sequence
          (:then_0
            (Default|ReadData (Variables|Default|GetSerial%20Com)))
          (:then_1
            (Class|ControlPawn|ChangeLightwithHardware (Variables|/Game/Blueprints/BP_SerialCom_v4_UE510.BP_SerialCom_v4_UE510_C|GetLightIndex (Variables|Default|GetSerial%20Com))))
          (:then_2
            (Class|ControlPawn|ChangeMapwithHardware (Variables|/Game/Blueprints/BP_SerialCom_v4_UE510.BP_SerialCom_v4_UE510_C|GetMapsIndex (Variables|Default|GetSerial%20Com))))
          (:then_3
            (Class|ControlPawn|ChangeMirrorwithHardware (Variables|/Game/Blueprints/BP_SerialCom_v4_UE510.BP_SerialCom_v4_UE510_C|GetButtonIndex (Variables|Default|GetSerial%20Com)))
            (return)))))))