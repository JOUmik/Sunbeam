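; BP_Beam is a light beam actor that follows the level's directional light and reacts to surfaces it hits.
; Every Tick it line-traces along the light direction and scales Niagara beams to the hit distance.
; Actor tags drive the response: Reflect spawns one bounce along the hit normal rather than a mirrored vector, Focal extends a lens beam, Water shows a caustic spotlight.
; Beam segments are pre-existing components, repositioned and rescaled.
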(event EventBeginPlay)

(event Collision|EventActorBeginOverlap
  (params (OtherActor :type Actor%20Object%20Reference)))

(event EventTick
  (params (DeltaSeconds :type Float%20%28single-precision%29))
  (bind _returnvalue (Transformation|GetActorLocation))
  (bind _cube1 (Variables|Default|GetCube1))
  (Variables|Default|SetHitWater false)
  (bind _outactors (Actor|GetAllActorsOfClass "/Script/Engine.DirectionalLight"))
  (Transformation|SetRelativeRotation (Variables|Default|GetCube) (Transformation|GetActorRotation (Utilities|Array|Get(acopy) _outactors)) false false)
  (Variables|Default|SetDirLightDir (Math|Vector|GetForwardVector (Transformation|GetActorRotation (Utilities|Array|Get(acopy) _outactors))))
  (bind (_hitobj _beamscale _hitnormal _hitactor _hitposition) (CallFunction|LightDetect _returnvalue (+ _returnvalue (* (Math|Vector|GetForwardVector (Transformation|GetActorRotation (Utilities|Array|Get(acopy) _outactors))) (Variables|Default|GetLightLength))) false))
  (Variables|Default|SetReflectRotation _hitnormal)
  (Variables|Default|SetDirLightHitPos _hitposition)
  (Niagara|SetNiagaraVariable(Vector3) (Variables|Default|GetNS_Beam) "BeamScale" _beamscale)
  (if _hitobj
    (CallFunction|HandleLightHit (Variables|/Script/Engine.Actor|GetTags _hitactor))
    (if (Variables|Default|GetHitReflectObj)
      (bind (_hitobj_2 _beamscale_2 _hitnormal_2 _hitactor_2 _hitposition_2) (CallFunction|LightDetect (Variables|Default|GetDirLightHitPos) (+ (Variables|Default|GetDirLightHitPos) (* (Variables|Default|GetReflectRotation) (Variables|Default|GetLightLength))) false _hitactor))
      (Transformation|SetWorldLocation _cube1 (Variables|Default|GetDirLightHitPos) false false)
      (Transformation|SetRelativeRotation _cube1 (Math|Conversions|RotationFromXVector (Variables|Default|GetReflectRotation)) false false)
      (Niagara|SetNiagaraVariable(Vector3) (Variables|Default|GetNS_Beam1) "BeamScale" _beamscale_2)
      (CallFunction|HandleLightHit (Variables|/Script/Engine.Actor|GetTags _hitactor_2))
      (CallFunction|AddFocalLight (Variables|Default|GetHitFocalLens) _hitposition_2 (Variables|Default|GetReflectRotation) false _hitactor_2)
      (CallFunction|AddCaustic (Variables|Default|GetHitWater) _hitposition_2 (Variables|Default|GetReflectRotation))
      (else
        (Niagara|SetNiagaraVariable(Vector3) (Variables|Default|GetNS_Beam1) "BeamScale" "0, 0, 0")
        (CallFunction|AddFocalLight (Variables|Default|GetHitFocalLens) (Variables|Default|GetDirLightHitPos) (Variables|Default|GetDirLightDir) false _hitactor)
        (CallFunction|AddCaustic (Variables|Default|GetHitWater) (Variables|Default|GetDirLightHitPos) (Variables|Default|GetDirLightDir))))))

(fn ConstructionScript
  (Niagara|SetNiagaraVariable(Vector3) (Variables|Default|GetNS_Beam) "BeamScale" (Variables|Default|GetIn%20Value)))

(fn LightDetect
  (params (StartPos :type Vector%20%28by%20ref%29) (EndPos :type Vector%20%28by%20ref%29) (DisplayTrace :type Boolean%20%28by%20ref%29) (IgnoreItem :type Actor%20Object%20Reference))
  (bind _lightsize (Variables|Default|GetLightSize))
  (if DisplayTrace
    (Variables|Default|SetDraw%20Debug%20Type "ForOneFrame")
    (else
      (Variables|Default|SetDraw%20Debug%20Type "None")))
  (bind (_outhit _returnvalue) (Collision|LineTraceForObjects StartPos EndPos (Utilities|Array|MakeArray "ObjectTypeQuery1") false (Utilities|Array|MakeArray IgnoreItem) (Variables|Default|GetDraw%20Debug%20Type)))
  (Variables|Default|SetHitReflectObj _returnvalue)
  (if _returnvalue
    (return (Variables|Default|GetHitReflectObj) (Math|Vector|MakeVector _lightsize _lightsize (+ (* (Math|Vector|Distance(Vector) (.ImpactPoint (Collision|BreakHitResult _outhit)) StartPos) 0.005) (Variables|Default|GetLightLengthPlus))) (.Normal (Collision|BreakHitResult _outhit)) (.HitActor (Collision|BreakHitResult _outhit)) (.ImpactPoint (Collision|BreakHitResult _outhit)))
    (else
      (return (Variables|Default|GetHitReflectObj) (Math|Vector|MakeVector _lightsize _lightsize 35.0) (.Normal (Collision|BreakHitResult _outhit)) (.HitActor (Collision|BreakHitResult _outhit)) (.ImpactPoint (Collision|BreakHitResult _outhit))))))

(fn AddFocalLight
  (params (HitFocal :type Boolean) (StartPoint :type Vector) (LightDirectionVector :type Vector) (DisplayTrace :type Boolean) (IgnoreItem :type Actor%20Object%20Reference))
  (bind _cubefocal (Variables|Default|GetCubeFocal))
  (if HitFocal
    (Variables|Default|SetStart%20Pos (+ StartPoint (* LightDirectionVector (Variables|Default|GetLensThickness))))
    (bind (_hitobj _beamscale) (CallFunction|LightDetect (Variables|Default|GetStart%20Pos) (+ StartPoint (* LightDirectionVector (Variables|Default|GetLightLength))) DisplayTrace IgnoreItem))
    (if _hitobj
      (Transformation|SetWorldLocation _cubefocal (Variables|Default|GetStart%20Pos) false false)
      (Transformation|SetRelativeRotation _cubefocal (Math|Conversions|RotationFromXVector LightDirectionVector) false false)
      (Niagara|SetNiagaraVariable(Vector3) (Variables|Default|GetNS_BeamFocal) "BeamScale" (Math|Vector|MakeVector 1.1 1.1 (- (.Z (Math|Vector|BreakVector _beamscale)) 9.0)))
      (else
        (Niagara|SetNiagaraVariable(Vector3) (Variables|Default|GetNS_BeamFocal) "BeamScale" "1.100000,1.100000,8.000000")))
    (else
      (Niagara|SetNiagaraVariable(Vector3) (Variables|Default|GetNS_BeamFocal) "BeamScale" "0.000000,0.000000,0.000000"))))

(fn HandleLightHit
  (params (Tags :type Array%20of%20Names))
  (Variables|Default|SetHitReflectObj false)
  (Variables|Default|SetHitFocalLens false)
  (for _array_element Tags
    (if (== _array_element "Reflect")
      (Variables|Default|SetHitReflectObj true)
      (elif (== _array_element "Focal")
        (Variables|Default|SetHitFocalLens true)
        (elif (== _array_element "Water")
          (Variables|Default|SetHitWater true))))))

(fn AddCaustic
  (params (HitWater :type Boolean) (Position :type Vector) (Rotation :type Vector))
  (bind _watercaustic (Variables|Default|GetWaterCaustic))
  (Rendering|SetVisibility (Variables|Default|GetSpotLight1) HitWater false)
  (Transformation|SetWorldLocation _watercaustic Position false false)
  (Transformation|SetRelativeRotation _watercaustic (Math|Conversions|RotationFromXVector Rotation) false false))