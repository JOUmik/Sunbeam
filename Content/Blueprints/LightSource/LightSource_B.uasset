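; LightSource_B is a lamp-like interactable light source that reports the LightSource.Moon tag and starts with its point light hidden.
; PlayBloomAnimForward activates the Niagara lamp effect, shows the light and sets bloom status to true.
; PlayBloomAnimReverse resets, pauses and deactivates the effect, hides the light and sets bloom status to false.
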(event EventBeginPlay
  (Rendering|SetVisibility (Variables|Default|GetPointLight) false false))

(event EventPlayBloomAnimForward
  (bind _ns_lamplight (Variables|Default|GetNS_LampLight))
  (Components|Activation|Activate _ns_lamplight false)
  (Components|Activation|SetActive _ns_lamplight true false)
  (Rendering|SetVisibility (Variables|Default|GetPointLight) true false)
  (Class|BeamFlowerBase|SetBloomStatus true))

(event EventPlayBloomAnimReverse
  (bind _ns_lamplight (Variables|Default|GetNS_LampLight))
  (Niagara|ResetSystem _ns_lamplight)
  (Class|NiagaraComponent|SetPaused _ns_lamplight true)
  (Components|Activation|SetActive _ns_lamplight false false)
  (Rendering|SetVisibility (Variables|Default|GetPointLight) false false)
  (Class|BeamFlowerBase|SetBloomStatus false))

(fn ConstructionScript)

(fn GetInteractableTags
  (return "(GameplayTags=((TagName=\"LightSource.Moon\")))"))