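; Flower actor that blooms permanently after enough continuous exposure to directional light.
; Each tick it line-traces against WorldStatic objects along the second found DirectionalLight's rotation axis, treating a hit as shade.
; The Cube's material switches between shaded and lit looks, while a one-second Delay in Tick increments an exposure counter that shade resets.
; Reaching TimeExposure sets the bloomed material and stops further checks.
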(event EventBeginPlay
  (Variables|Default|SetLighted false)
  (Variables|Default|SetBloomed false)
  (Variables|Default|SetIndex 0)
  (Variables|Default|SetCounted false))

(event Collision|EventActorBeginOverlap
  (params (OtherActor :type Actor%20Object%20Reference)))

(event EventTick
  (params (DeltaSeconds :type Float%20%28single-precision%29))
  (bind _returnvalue (Transformation|GetActorLocation))
  (if (not (Variables|Default|GetBloomed))
    (bind _outactors (Actor|GetAllActorsOfClass "/Script/Engine.DirectionalLight"))
    (bind (_outhit _returnvalue_2) (Collision|LineTraceForObjects _returnvalue (+ _returnvalue (* (* (Math|Vector|GetForwardVector (Transformation|GetActorRotation (Utilities|Array|Get(acopy) _outactors 1))) (Variables|Default|GetTraceLength)) (Variables|Default|GetLengthUnit))) (Utilities|Array|MakeArray "ObjectTypeQuery1") false 0 "None"))
    (if _returnvalue_2
      (Rendering|Material|SetMaterial (Variables|Default|GetCube) 0 "/Game/Materials/MI_flower.MI_flower")
      (Variables|Default|SetLighted false)
      (else
        (Rendering|Material|SetMaterial (Variables|Default|GetCube) 0 "/Game/Materials/MI_flower_bloom.MI_flower_bloom")
        (Variables|Default|SetLighted true)))
    (if (Variables|Default|GetLighted)
      (Utilities|FlowControl|Delay 1.0)
      (bind _output_get (Variables|Default|SetIndex (+ (Variables|Default|GetIndex) 1)))
      (else
        (Variables|Default|SetIndex 0)))
    (if (>= _output_get (Variables|Default|GetTime_Exposure))
      (Variables|Default|SetBloomed true)
      (Rendering|Material|SetMaterial (Variables|Default|GetCube) 0 "/Game/Materials/MI_flower_bloomed.MI_flower_bloomed"))))

(fn ConstructionScript)