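; Flower actor that blooms when exposed to directional light and stays bloomed after enough accumulated exposure.
; While the control pawn's light index is zero, Tick line-traces along the second directional light's direction; a hit resets exposure, a clear path adds time through a Delay.
; Exposure changes call PlayFlower, whose FlipFlops play or reverse six geometry caches and a Timeline scaling them and the plant mesh.
; A status mesh swaps materials per state.
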(event Custom|PlayFlower
  (bind _geometrycache (Variables|Default|GetGeometryCache))
  (bind _s_butterfly_weed_vkblbcdia_var10_lod1 (Variables|Default|GetS_Butterfly_Weed_vkblbcdia_Var10_lod1))
  (bind _returnvalue (Transformation|GetWorldTransform _s_butterfly_weed_vkblbcdia_var10_lod1))
  (Utilities|FlowControl|Sequence
    (:then_0
      (Utilities|FlowControl|FlipFlop
        (:A
          (Audio|Components|Audio|Play _geometrycache))
        (:B
          (Class|GeometryCacheComponent|PlayReversed _geometrycache))))
    (:then_1
      (Utilities|FlowControl|FlipFlop
        (:A
          (bind (_direction _newtrack_0 _newtrack_1 _newtrack_2) (Timeline|Timeline Play)
            (:Update
              (Transformation|SetWorldScale3D _geometrycache (* _newtrack_0 (Variables|Default|GetFlower_Scale_0)))
              (Transformation|SetWorldScale3D (Variables|Default|GetGeometryCache1) (* _newtrack_0 (Variables|Default|GetFlower_Scale_1)))
              (Transformation|SetWorldScale3D (Variables|Default|GetGeometryCache2) (* _newtrack_0 (Variables|Default|GetFlower_Scale_2)))
              (Transformation|SetWorldScale3D (Variables|Default|GetGeometryCache3) (* _newtrack_0 (Variables|Default|GetFlower_Scale_3)))
              (Transformation|SetWorldScale3D (Variables|Default|GetGeometryCache4) (* _newtrack_0 (Variables|Default|GetFlower_Scale_4)))
              (Transformation|SetWorldScale3D (Variables|Default|GetGeometryCache5) (* _newtrack_0 (Variables|Default|GetFlower_Scale_5)))
              (Transformation|SetWorldTransform _s_butterfly_weed_vkblbcdia_var10_lod1 (Math|Transform|MakeTransform (.location _returnvalue) (.rotation _returnvalue) (* (Math|Vector|MakeVector _newtrack_1 _newtrack_1 _newtrack_2) (Variables|Default|GetScale))) false false))
            (:Finished
              (Sequencer|Player|Pause _geometrycache))))
        (:B
          (Timeline|Timeline Reverse))))))

(event EventBeginPlay
  (Variables|Default|SetLighted false)
  (Variables|Default|SetBloomed false)
  (Variables|Default|SetCurrentTime 0.0)
  (Variables|Default|SetCounted false)
  (if (Utilities|Operators|EqualEqual :A (Variables|Default|GetScale))
    (Variables|Default|SetScale (.scale (Transformation|GetWorldTransform (Variables|Default|GetS_Butterfly_Weed_vkblbcdia_Var10_lod1))))
    (Variables|Default|SetFlower_Scale_0 (.scale (Transformation|GetWorldTransform (Variables|Default|GetGeometryCache))))
    (Variables|Default|SetFlower_Scale_1 (.scale (Transformation|GetWorldTransform (Variables|Default|GetGeometryCache1))))
    (Variables|Default|SetFlower_Scale_2 (.scale (Transformation|GetWorldTransform (Variables|Default|GetGeometryCache2))))
    (Variables|Default|SetFlower_Scale_3 (.scale (Transformation|GetWorldTransform (Variables|Default|GetGeometryCache3))))
    (Variables|Default|SetFlower_Scale_4 (.scale (Transformation|GetWorldTransform (Variables|Default|GetGeometryCache4))))
    (Variables|Default|SetFlower_Scale_5 (.scale (Transformation|GetWorldTransform (Variables|Default|GetGeometryCache5))))))

(event EventTick
  (params (DeltaSeconds :type Float%20%28single-precision%29))
  (bind _duration (Variables|Default|GetDuration))
  (bind _staticmesh (Variables|Default|GetStaticMesh))
  (bind _returnvalue (Transformation|GetWorldLocation _staticmesh))
  (bind _returnvalue_2 (Actor|GetActorOfClass "/Game/Blueprints/BP_ControlPawn.BP_ControlPawn_C"))
  (if (== (Variables|/Script/Sunbeam.ControlPawn|GetEnabledLightIndex _returnvalue_2) 0)
    (if (not (Variables|Default|GetBloomed))
      (bind _outactors (Actor|GetAllActorsOfClass "/Script/Engine.DirectionalLight"))
      (bind (_outhit _returnvalue_3) (Collision|LineTraceForObjects _returnvalue (+ _returnvalue (* (* (Math|Vector|GetForwardVector (Transformation|GetActorRotation (Utilities|Array|Get(acopy) _outactors 1))) (Variables|Default|GetTraceLength)) (Variables|Default|GetLengthUnit))) (Utilities|Array|MakeArray "ObjectTypeQuery1") false 0 "None"))
      (if _returnvalue_3
        (Rendering|Material|SetMaterial (Variables|Default|GetStaticMesh) 0 "/Game/Materials/MI_flower.MI_flower")
        (if (!= (Variables|Default|GetCurrentTime) 0.0)
          (CallFunction|PlayFlower))
        (Variables|Default|SetCurrentTime 0.0)
        (else
          (Rendering|Material|SetMaterial (Variables|Default|GetStaticMesh) 0 "/Game/Materials/MI_flower_bloom.MI_flower_bloom")
          (Utilities|FlowControl|Delay _duration)
          (if (== (Variables|Default|GetCurrentTime) 0.0)
            (CallFunction|PlayFlower))
          (bind _output_get (Variables|Default|SetCurrentTime (+ _duration (Variables|Default|GetCurrentTime))))))
      (if (>= _output_get (Variables|Default|GetTime_Exposure))
        (Variables|Default|SetBloomed true)
        (Rendering|Material|SetMaterial (Variables|Default|GetStaticMesh) 0 "/Game/Materials/MI_flower_bloomed.MI_flower_bloomed")
        (Variables|Default|SetCurrentTime 0.0)))))

(fn ConstructionScript)