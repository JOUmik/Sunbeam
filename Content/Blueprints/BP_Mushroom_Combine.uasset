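; BP_Mushroom_Combine is a mushroom that blooms after enough exposure to the directional light.
; While BP_ControlPawn's EnabledLightIndex is 1, Tick traces along the light's forward axis to detect blockers.
; Unblocked time accumulates through a Delay until TimeExposure locks the bloomed state, while blocking resets it.
; Exposure changes swap flower materials and flip-flop the GeometryCache animation and scale timeline between forward and reverse.
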(event Custom|PlayMushroom
  (bind _geometrycache (Variables|Default|GetGeometryCache))
  (Utilities|FlowControl|Sequence
    (:then_0
      (Utilities|FlowControl|FlipFlop
        (:A
          (Audio|Components|Audio|Play _geometrycache))
        (:B
          (Class|GeometryCacheComponent|PlayReversed _geometrycache))))
    (:then_1
      (Utilities|FlowControl|FlipFlop
        (:A
          (bind _newtrack_0 (Timeline|Timeline Play)
            (:Update
              (Transformation|SetWorldScale3D _geometrycache (* _newtrack_0 (Variables|Default|GetScale))))
            (:Finished
              (Sequencer|Player|Pause _geometrycache))))
        (:B
          (Timeline|Timeline Reverse))))))

(event EventBeginPlay
  (Variables|Default|SetLighted false)
  (Variables|Default|SetBloomed false)
  (Variables|Default|SetCurrentTime 0.0)
  (Variables|Default|SetCounted false)
  (if (Utilities|Operators|EqualEqual :A (Variables|Default|GetScale))
    (Variables|Default|SetScale (.scale (Transformation|GetWorldTransform (Variables|Default|GetGeometryCache))))))

(event EventTick
  (params (DeltaSeconds :type Float%20%28single-precision%29))
  (bind _duration (Variables|Default|GetDuration))
  (bind _staticmesh (Variables|Default|GetStaticMesh))
  (bind _returnvalue (Transformation|GetWorldLocation _staticmesh))
  (bind _returnvalue_2 (Actor|GetActorOfClass "/Game/Blueprints/BP_ControlPawn.BP_ControlPawn_C"))
  (if (== (Variables|/Script/Sunbeam.ControlPawn|GetEnabledLightIndex _returnvalue_2) 1)
    (if (not (Variables|Default|GetBloomed))
      (bind _outactors (Actor|GetAllActorsOfClass "/Script/Engine.DirectionalLight"))
      (bind (_outhit _returnvalue_3) (Collision|LineTraceForObjects _returnvalue (+ _returnvalue (* (* (Math|Vector|GetForwardVector (Transformation|GetActorRotation (Utilities|Array|Get(acopy) _outactors))) (Variables|Default|GetTraceLength)) (Variables|Default|GetLengthUnit))) (Utilities|Array|MakeArray "ObjectTypeQuery1") false 0 "None"))
      (if _returnvalue_3
        (Rendering|Material|SetMaterial (Variables|Default|GetStaticMesh) 0 "/Game/Materials/MI_flower.MI_flower")
        (if (!= (Variables|Default|GetCurrentTime) 0.0)
          (CallFunction|PlayMushroom))
        (Variables|Default|SetCurrentTime 0.0)
        (else
          (Rendering|Material|SetMaterial (Variables|Default|GetStaticMesh) 0 "/Game/Materials/MI_flower_bloom.MI_flower_bloom")
          (Utilities|FlowControl|Delay _duration)
          (if (== (Variables|Default|GetCurrentTime) 0.0)
            (CallFunction|PlayMushroom))
          (bind _output_get (Variables|Default|SetCurrentTime (+ _duration (Variables|Default|GetCurrentTime))))))
      (if (>= _output_get (Variables|Default|GetTime_Exposure))
        (Variables|Default|SetBloomed true)
        (Rendering|Material|SetMaterial (Variables|Default|GetStaticMesh) 0 "/Game/Materials/MI_flower_bloomed.MI_flower_bloomed")
        (Variables|Default|SetCurrentTime 0.0)))))

(fn ConstructionScript)