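; BP_Paint_Room is an interactable painting object that switches between bloomed and unbloomed states.
; Forward and reverse bloom events set the playing and bloom status, toggle and reset a Niagara effect, and swap the large painting mesh's material.
; Each event also drives the FMOD parameter Track3_1 through its own timeline, played from start or reversed from end.
; The Niagara effect starts hidden on BeginPlay.
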(event EventBeginPlay
  (Development|SetHiddeninGame (Variables|Default|GetNiagara) true false))

(event EventPlayBloomAnimForward
  (bind _niagara (Variables|Default|GetNiagara))
  (Variables|Default|SetbIsPlaying true)
  (Class|BeamObjective|SetBloomStatus true)
  (Development|SetHiddeninGame _niagara false false)
  (Niagara|ResetSystem _niagara)
  (Rendering|Material|SetMaterial (Variables|Default|GetSM_Painting_Large) 0 "/Game/Models/Zeyang/Colored_Painting_texture/M_Painting.M_Painting")
  (bind _newtrack_0 (Timeline|Timeline PlayFromStart)
    (:Update
      (Class|FMODAudioComponent|SetParameter (Variables|Default|GetFMODAudio) "Track3_1" _newtrack_0))))

(event EventPlayBloomAnimReverse
  (bind _niagara (Variables|Default|GetNiagara))
  (Variables|Default|SetbIsPlaying false)
  (Class|BeamObjective|SetBloomStatus false)
  (Development|SetHiddeninGame _niagara true false)
  (Niagara|ResetSystem _niagara)
  (Rendering|Material|SetMaterial (Variables|Default|GetSM_Painting_Large) 0 "/Game/Models/Zeyang/Room_Interior/Texture_Group_2/M_Texsture_Group_2.M_Texsture_Group_2")
  (bind _newtrack_0 (Timeline|Timeline_0 ReverseFromEnd)
    (:Update
      (Class|FMODAudioComponent|SetParameter (Variables|Default|GetFMODAudio) "Track3_1" _newtrack_0))))

(fn ConstructionScript)