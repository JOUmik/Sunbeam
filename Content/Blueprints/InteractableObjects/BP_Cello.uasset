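; BP_Cello is an interactable cello that shows a Niagara effect while a specific light source interacts with it.
; The effect starts hidden, appears on interact begin only if the light source's display name is "BP_SunBeam0", and hides on interact end.
; The light check is a hardcoded name comparison, while the reported response tag is LightSource.Moon.
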(event EventBeginPlay
  (Development|SetHiddeninGame (Variables|Default|GetNiagara) true false))

(event Collision|EventActorBeginOverlap
  (params (OtherActor :type Actor%20Object%20Reference)))

(event EventOnBeginInteract
  (params (LightHitResult :type Hit%20Result%20Structure) (LightSource :type Actor%20Object%20Reference))
  (if (Utilities|Enum|Equal(Enum) (Utilities|GetDisplayName LightSource) "BP_SunBeam0")
    (Development|SetHiddeninGame (Variables|Default|GetNiagara) false false)))

(event EventOnEndInteract
  (Development|SetHiddeninGame (Variables|Default|GetNiagara) true false))

(fn ConstructionScript)

(fn GetInteractableResponseTags
  (return "(GameplayTags=((TagName=\"LightSource.Moon\"),(TagName=\"LightSource.Sun\")))"))