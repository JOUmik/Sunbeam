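; Interactable music box actor that spins its handle and figure while bloomed.
; PlayBloomAnimForward and PlayBloomAnimReverse toggle IsPlaying and pass the same state to SetBloomStatus.
; Tick accumulates elapsed time and, while playing, rolls Handle and yaws Guy by RotationSpeed each time RotateFrequency is exceeded, giving stepped rather than frame-rate-driven rotation.
; The graph contains no audio playback, and a duplicate rotation branch is left unconnected.
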(event EventBeginPlay)

(event Collision|EventActorBeginOverlap
  (params (OtherActor :type Actor%20Object%20Reference)))

(event EventTick
  (params (DeltaSeconds :type Float%20%28single-precision%29))
  (bind _output_get (Variables|Default|SetTimeElapsed (+ DeltaSeconds (Variables|Default|GetTimeElapsed))))
  (if (> (- _output_get (Variables|Default|GetLastPlayTime)) (Variables|Default|GetRotateFrequency))
    (Variables|Default|SetLastPlayTime (Variables|Default|GetTimeElapsed))
    (if (Variables|Default|GetbIsPlaying)
      ;[1 1 1] Rotate the music box
      (Transformation|AddRelativeRotation (Variables|Default|GetHandle) (Math|Rotator|MakeRotator (Variables|Default|GetRotationSpeed) 0.0 0.0) false false)
      (Transformation|AddRelativeRotation (Variables|Default|GetGuy) (Math|Rotator|MakeRotator 0.0 0.0 (Variables|Default|GetRotationSpeed)) false false))))

(event EventPlayBloomAnimForward
  (Variables|Default|SetbIsPlaying true)
  (Class|BeamObjective|SetBloomStatus true))

(event EventPlayBloomAnimReverse
  (Variables|Default|SetbIsPlaying false)
  (Class|BeamObjective|SetBloomStatus false))

(fn ConstructionScript)