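; Music box interactable that turns on and off through forward and reverse bloom animation events.
; Each event sets the playing flag and bloom status, shows or hides and resets the Niagara effect, and runs its own timeline to drive the FMOD Track3_4 parameter.
; While playing, Tick rotates the handle and guy components in fixed steps on a timer set by RotateFrequency, without scaling by delta time.
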(event EventBeginPlay
  (Development|SetHiddeninGame (Variables|Default|GetNiagara) true false))

(event Collision|EventActorBeginOverlap
  (params (OtherActor :type Actor%20Object%20Reference)))

(event EventTick
  (params (DeltaSeconds :type Float%20%28single-precision%29))
  (bind _output_get (Variables|Default|SetTimeElapsed (+ DeltaSeconds (Variables|Default|GetTimeElapsed))))
  (if (and (> _output_get (Variables|Default|GetRotateFrequency)) (Variables|Default|GetbIsPlaying))
    ;[1 1 1] Rotate the music box
    (Transformation|AddRelativeRotation (Variables|Default|GetHandle) (Math|Rotator|MakeRotator (Variables|Default|GetRotationSpeed) 0.0 0.0) false false)
    (Transformation|AddRelativeRotation (Variables|Default|GetGuy) (Math|Rotator|MakeRotator 0.0 0.0 (Variables|Default|GetRotationSpeed)) false false)
    (Variables|Default|SetTimeElapsed 0.0)))

(event EventPlayBloomAnimForward
  (bind _niagara (Variables|Default|GetNiagara))
  (Variables|Default|SetbIsPlaying true)
  (Class|BeamObjective|SetBloomStatus true)
  (Development|SetHiddeninGame _niagara false false)
  (Niagara|ResetSystem _niagara)
  (bind _newtrack_0 (Timeline|Timeline PlayFromStart)
    (:Update
      (Class|FMODAudioComponent|SetParameter (Variables|Default|GetFMODAudio) "Track3_4" _newtrack_0))))

(event EventPlayBloomAnimReverse
  (bind _niagara (Variables|Default|GetNiagara))
  (Variables|Default|SetbIsPlaying false)
  (Class|BeamObjective|SetBloomStatus false)
  (Development|SetHiddeninGame _niagara true false)
  (Niagara|ResetSystem _niagara)
  (bind _newtrack_0 (Timeline|Timeline_0 ReverseFromEnd)
    (:Update
      (Class|FMODAudioComponent|SetParameter (Variables|Default|GetFMODAudio) "Track3_4" _newtrack_0))))

(fn ConstructionScript)