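; Interactable bush that responds to light sources, toggling its bloom status and a day-symbol effect.
; Begin and end interact events keep a running count of active light sources, and the effect starts paused on BeginPlay.
; Interaction unpauses the effect at a non-negative count and pauses it again below one.
; Bloom switches on when the count rises to one and off when it falls to zero, so overlapping sources do not retrigger it.
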(event EventBeginPlay
  (Class|NiagaraComponent|SetPaused (Variables|Default|GetNS_Symbol_Day) true))

(event EventOnEndInteract
  (bind _output_get (Variables|Components|SetCurLightSourceCount (+ (Variables|Components|GetCurLightSourceCount) -1)))
  (if (< _output_get 1)
    (Class|NiagaraComponent|SetPaused (Variables|Default|GetNS_Symbol_Day) true)
    (if (== (Variables|Components|GetCurLightSourceCount) 0)
      (Class|BeamObjective|SetBloomStatus false))))

(event EventOnBeginInteract
  (params (LightHitResult :type Hit%20Result%20Structure) (LightSource :type Actor%20Object%20Reference))
  (bind _output_get (Variables|Components|SetCurLightSourceCount (+ (Variables|Components|GetCurLightSourceCount) 1)))
  (if (>= _output_get 0)
    (Class|NiagaraComponent|SetPaused (Variables|Default|GetNS_Symbol_Day) false)
    (if (== (Variables|Components|GetCurLightSourceCount) 1)
      (Class|BeamObjective|SetBloomStatus true))))

(fn ConstructionScript)