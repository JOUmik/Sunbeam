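; BP_Phonograph is an interactable phonograph that switches between idle and playing states, with a spinning disk and a Niagara effect.
; PlayBloomAnimForward and PlayBloomAnimReverse set the playing flag and bloom status, show or hide the effect, and reset its system.
; While playing, Tick adds a fixed yaw step to the disk every frame, without delta-time scaling.
; The effect starts hidden on BeginPlay.
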(event EventBeginPlay
  (Development|SetHiddeninGame (Variables|Default|GetNiagara) true false))

(event Collision|EventActorBeginOverlap
  (params (OtherActor :type Actor%20Object%20Reference)))

(event EventTick
  (params (DeltaSeconds :type Float%20%28single-precision%29))
  (if (Variables|Default|GetbIsPlaying)
    (Transformation|AddRelativeRotation (Variables|Default|Getdisk) (Math|Rotator|MakeRotator 0.0 0.0 (Variables|Default|GetRotationSpeed)) false false)))

(event EventPlayBloomAnimForward
  (bind _niagara (Variables|Default|GetNiagara))
  (Variables|Default|SetbIsPlaying true)
  (Class|BeamObjective|SetBloomStatus true)
  (Development|SetHiddeninGame _niagara false false)
  (Niagara|ResetSystem _niagara))

(event EventPlayBloomAnimReverse
  (bind _niagara (Variables|Default|GetNiagara))
  (Variables|Default|SetbIsPlaying false)
  (Class|BeamObjective|SetBloomStatus false)
  (Development|SetHiddeninGame _niagara true false)
  (Niagara|ResetSystem _niagara))

(fn ConstructionScript)