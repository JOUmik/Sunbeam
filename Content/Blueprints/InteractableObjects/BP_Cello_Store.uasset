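; BP_Cello_Store is an interactable cello object that toggles a bloom state with a particle effect and a music layer.
; Forward and reverse bloom events set the playing flag and bloom status, then show or hide and reset the Niagara system, which starts hidden.
; Each event runs its own timeline, played forward or in reverse, to drive the FMOD Track3_2 parameter.
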(event EventBeginPlay
  (Development|SetHiddeninGame (Variables|Default|GetNiagara) true false))

(event EventPlayBloomAnimForward
  (bind _niagara (Variables|Default|GetNiagara))
  (Variables|Default|SetbIsPlaying true)
  (Class|BeamObjective|SetBloomStatus true)
  (Development|SetHiddeninGame _niagara false false)
  (Niagara|ResetSystem _niagara)
  (bind _newtrack_0 (Timeline|Timeline PlayFromStart)
    (:Update
      (Class|FMODAudioComponent|SetParameter (Variables|Default|GetFMODAudio) "Track3_2" _newtrack_0))))

(event EventPlayBloomAnimReverse
  (bind _niagara (Variables|Default|GetNiagara))
  (Variables|Default|SetbIsPlaying false)
  (Class|BeamObjective|SetBloomStatus false)
  (Development|SetHiddeninGame _niagara true false)
  (Niagara|ResetSystem _niagara)
  (bind _newtrack_0 (Timeline|Timeline_0 ReverseFromEnd)
    (:Update
      (Class|FMODAudioComponent|SetParameter (Variables|Default|GetFMODAudio) "Track3_2" _newtrack_0))))

(fn ConstructionScript)