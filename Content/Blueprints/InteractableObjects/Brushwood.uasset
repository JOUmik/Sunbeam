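; Brushwood is an interactable object whose NSSymbolDay effect runs while light sources interact with it.
; The effect starts paused, and interact begin and end events adjust a light source counter.
; Beginning an interaction unpauses the effect, and ending one pauses it again once the count drops below one.
; It reports the SecondarySource.Sunflower tag as its interactable tag.
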(event EventBeginPlay
  (Class|NiagaraComponent|SetPaused (Variables|Default|GetNS_Symbol_Day) true))

(event EventOnEndInteract
  (bind _output_get (Variables|Components|SetCurLightSourceCount (+ (Variables|Components|GetCurLightSourceCount) -1)))
  (if (< _output_get 1)
    (Class|NiagaraComponent|SetPaused (Variables|Default|GetNS_Symbol_Day) true)))

(event EventOnBeginInteract
  (params (LightHitResult :type Hit%20Result%20Structure) (LightSource :type Actor%20Object%20Reference))
  (bind _output_get (Variables|Components|SetCurLightSourceCount (+ (Variables|Components|GetCurLightSourceCount) 1)))
  (if (>= _output_get 0)
    (Class|NiagaraComponent|SetPaused (Variables|Default|GetNS_Symbol_Day) false)))

(fn ConstructionScript)

(fn GetInteractableTags
  (return "(GameplayTags=((TagName=\"SecondarySource.Sunflower\"),(TagName=\"LightSource.Sun\")))"))