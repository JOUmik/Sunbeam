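; BP_Tombstone is an interactable tombstone that switches between a bloomed and an unbloomed state.
; Its forward and reverse bloom events set the playing and bloom flags, toggle and reset a Niagara effect that starts hidden, and swap the stone's material to show or remove text.
; The same events turn the FMOD Track_2 parameter on or off, so audio follows the bloom state.
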(event EventBeginPlay
  (Development|SetHiddeninGame (Variables|Default|GetNiagara) true false))

(event EventPlayBloomAnimForward
  (bind _niagara (Variables|Default|GetNiagara))
  (Variables|Default|SetbIsPlaying true)
  (Class|BeamObjective|SetBloomStatus true)
  (Development|SetHiddeninGame _niagara false false)
  (Niagara|ResetSystem _niagara)
  (Rendering|Material|SetMaterial (Variables|Default|GetTombVar1) 0 "/Game/Models/Mingyuan/Moldel_Map/Mat/M_TombVar1WithText.M_TombVar1WithText")
  (Class|FMODAudioComponent|SetParameter (Variables|Default|GetFMODAudio) "Track_2" 1.0))

(event EventPlayBloomAnimReverse
  (bind _niagara (Variables|Default|GetNiagara))
  (Variables|Default|SetbIsPlaying false)
  (Class|BeamObjective|SetBloomStatus false)
  (Development|SetHiddeninGame _niagara true false)
  (Niagara|ResetSystem _niagara)
  (Rendering|Material|SetMaterial (Variables|Default|GetTombVar1) 0 "/Game/Models/Mingyuan/Moldel_Map/Mat/TombVar1_mat2.TombVar1_mat2")
  (Class|FMODAudioComponent|SetParameter (Variables|Default|GetFMODAudio) "Track_2" 0.0))

(fn ConstructionScript)