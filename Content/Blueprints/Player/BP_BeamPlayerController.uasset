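; Player controller for a light-beam game that can take input from physical hardware over a serial link.
; When hardware use is enabled, BPReadDate polls the BP_SerialCom actor and passes its light, button and level-rotation indices to handlers defined outside this graph.
; ChangeMirror and ChangeLightBeam events look up BP_Beam to set its focal model or sunbeam color.
; Hardware map switching is present but left unconnected.
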(event EventBeginPlay)

(event EventTick
  (params (DeltaSeconds :type Float%20%28single-precision%29)))

(event EventChangeLightBeam
  (bind _returnvalue (Actor|GetActorOfClass "/Game/Blueprints/BP_Beam.BP_Beam_C"))
  (Utilities|IsValid _returnvalue
    (:Is%20Valid
      (Default|SetSunbeamColor _returnvalue))))

(event EventChangeMirror
  (params (bShow :type Boolean))
  (bind _returnvalue (Actor|GetActorOfClass "/Game/Blueprints/BP_Beam.BP_Beam_C"))
  (Utilities|IsValid _returnvalue
    (:Is%20Valid
      (Default|SetFocalModel _returnvalue bShow))))

(event EventBPReadDate
  (if (Variables|Default|GetUseHardware)
    (bind _returnvalue (Actor|GetActorOfClass "/Game/Blueprints/BP_SerialCom_v4_UE510.BP_SerialCom_v4_UE510_C"))
    (Utilities|IsValid _returnvalue
      (:Is%20Valid
        (Variables|Default|SetSerial%20Com _returnvalue)
        (Utilities|FlowControl|Sequence
          (:then_0
            (Default|ReadData (Variables|Default|GetSerial%20Com)))
          (:then_1
            (Class|BeamPlayerController|SwitchBeamState (Variables|/Game/Blueprints/BP_SerialCom_v4_UE510.BP_SerialCom_v4_UE510_C|GetLightIndex (Variables|Default|GetSerial%20Com))))
          (:then_3
            (Class|BeamPlayerController|ChangeMirrorwithHardware (Variables|/Game/Blueprints/BP_SerialCom_v4_UE510.BP_SerialCom_v4_UE510_C|GetButtonIndex (Variables|Default|GetSerial%20Com))))
          (:then_4
            (Class|BeamPlayerController|RotateLevelwithHardware (Variables|/Game/Blueprints/BP_SerialCom_v4_UE510.BP_SerialCom_v4_UE510_C|GetRotateLevelIndex (Variables|Default|GetSerial%20Com)))))))))

(fn ConstructionScript)