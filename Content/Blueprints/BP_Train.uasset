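; BP_Train is an actor that shuttles back and forth along the world Y axis.
; Tick passes through a short Delay, then offsets the location by Speed without sweeping, with the Left flag choosing the sign.
; A Timer grows by a fixed increment per step and flips Left at a threshold, so travel depends on frame rate rather than delta time.
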(event EventBeginPlay)

(event Collision|EventActorBeginOverlap
  (params (OtherActor :type Actor%20Object%20Reference)))

(event EventTick
  (params (DeltaSeconds :type Float%20%28single-precision%29))
  (Utilities|FlowControl|Delay 0.01)
  (if (Variables|Default|Getleft)
    (Transformation|SetActorLocation (+ (Transformation|GetActorLocation) (Math|Vector|MakeVector 0.0 (Variables|Default|GetSpeed) 0.0)) false false)
    (bind _output_get (Variables|Default|Settimer (+ (Variables|Default|Gettimer) 0.01)))
    (if (>= _output_get 4.0)
      (Variables|Default|Setleft false)
      (Variables|Default|Settimer 0.0))
    (else
      (Transformation|SetActorLocation (+ (Transformation|GetActorLocation) (Math|Vector|MakeVector 0.0 (* (Variables|Default|GetSpeed) -1.0) 0.0)) false false)
      (bind _output_get_2 (Variables|Default|Settimer (+ (Variables|Default|Gettimer) 0.01)))
      (if (>= _output_get_2 4.0)
        (Variables|Default|Setleft true)
        (Variables|Default|Settimer 0.0)))))

(fn ConstructionScript)