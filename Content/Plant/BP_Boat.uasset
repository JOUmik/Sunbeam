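; BP_Boat moves an array of boat components along a spline as a looping train while its Switch flag is on.
; Each Tick advances a shared Distance by Speed once per array element, placing each boat at an index-based TrainLength offset.
; Boats take the spline's location and rotation, a uniform BoatScale and a fixed local rotation correction.
; Distance resets to zero when any boat's offset position passes a hardcoded limit.
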(event EventBeginPlay)

(event Collision|EventActorBeginOverlap
  (params (OtherActor :type Actor%20Object%20Reference)))

(event EventTick
  (params (DeltaSeconds :type Float%20%28single-precision%29))
  (bind _boat_scale (Variables|Default|GetBoat_Scale))
  (if (Variables|Default|GetSwitch)
    (for (_array_element _array_index) (Utilities|Array|MakeArray (Variables|Default|GetBoat))
      (bind _output_get (Variables|Default|SetDistance (+ (* DeltaSeconds (Variables|Default|GetSpeed)) (Variables|Default|GetDistance))))
      (Transformation|SetWorldTransform _array_element (Math|Transform|MakeTransform (.location (Spline|GetTransformatDistanceAlongSpline (Variables|Default|GetSpline) (+ _output_get (* _array_index (Variables|Default|GetTrain_Length))) "World" false)) (.rotation (Spline|GetTransformatDistanceAlongSpline (Variables|Default|GetSpline) (+ _output_get (* _array_index (Variables|Default|GetTrain_Length))) "World" false)) (Math|Conversions|ToVector(Float) _boat_scale)) false false)
      (Class|SceneComponent|AddLocalTransform _array_element (Math|Transform|MakeTransform "0, 0, 0" "0.000000,270.000000,0.000000" (Math|Conversions|ToVector(Float) _boat_scale)) false false)
      (if (>= (+ _output_get (* _array_index (Variables|Default|GetTrain_Length))) 5.95e+03)
        (Variables|Default|SetDistance 0.0)))))

(fn ConstructionScript)