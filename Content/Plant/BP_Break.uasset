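; Mouse-click destruction tool that spawns a strain field where the player clicks in the world.
; BeginPlay shows the cursor, and each left click line-traces from the deprojected mouse position on the Visibility channel, with debug drawing.
; An FS_MasterField actor spawns at the hit location without a hit check and receives this Blueprint's StrainMagnitude.
; A disconnected branch that would move the Cube component to the hit point never runs.
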(event EventBeginPlay
  (Variables|/Script/Engine.PlayerController|SetbShowMouseCursor (Game|GetPlayerController 0) true))

(event Collision|EventActorBeginOverlap
  (params (OtherActor :type Actor%20Object%20Reference)))

(event EventTick
  (params (DeltaSeconds :type Float%20%28single-precision%29)))

(event Input|MouseEvents|LeftMouseButton
  (params (Key :type Key%20Structure :default "None"))
  (bind _returnvalue (Game|GetPlayerController 0))
  (bind (_worldlocation _worlddirection) (Game|Player|ConvertMouseLocationToWorldSpace _returnvalue))
  (:Pressed
    (bind _outhit (Collision|LineTraceByChannel _worldlocation (+ _worldlocation (* _worlddirection 5e+03)) "TraceTypeQuery1" false 0 "ForDuration"))
    (bind _returnvalue_2 (Game|SpawnActorfromClass "/Game/Plant/FS_MasterField_a.FS_MasterField_a_C" (Math|Transform|MakeTransform (.Location (Collision|BreakHitResult _outhit)) "0, 0, 0" "1.500000,1.500000,1.500000") "Undefined" "MultiplyWithRoot" 0 0))
    (Variables|/Game/Plant/FS_MasterField_a.FS_MasterField_a_C|SetStrain%20Magnitude _returnvalue_2 (Variables|Default|GetStrain_Magnitude))
    (Development|PrintString "OUT")))

(fn ConstructionScript)