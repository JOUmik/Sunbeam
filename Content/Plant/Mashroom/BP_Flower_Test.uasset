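; Test flower Blueprint that plays a GeometryCache animation forward or backward, toggled by the P key.
; The animation stays paused until the first press, then each press flips the Light flag that sets the playback direction.
; Tick counts frames itself, one per tick rather than by time, and pauses the cache at either end of the range.
; Timeline-driven scale and height changes are present but never run.
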(event EventBeginPlay)

(event EventTick
  (params (DeltaSeconds :type Float%20%28single-precision%29))
  (bind _geometrycache (Variables|Default|GetGeometryCache))
  (bind _geometrycache_2 (Variables|Default|GetGeometryCache))
  (if (not (Variables|Default|Getstart_Origin))
    (if (not (Variables|Default|GetPause))
      (Sequencer|Player|Pause (Variables|Default|GetGeometryCache))
      (Variables|Default|SetPause true))
    (elif (Variables|Default|Getlight)
      (if (Variables|Default|Getplay)
        (if (>= (Variables|Default|Getframe) 2.4e+02)
          (Variables|Default|Setframe 241.0)
          (if (not (Variables|Default|GetPause))
            (Sequencer|Player|Pause _geometrycache_2)
            (Variables|Default|SetPause true)
            (Variables|Default|Setre false))
          (else
            (Variables|Default|Setframe (+ (Variables|Default|Getframe) 1.0))))
        (else
          (Audio|Components|Audio|Play _geometrycache)
          (Variables|Default|Setplay true)
          (Variables|Default|SetPause false)
          (Variables|Default|Setre false)))
      (elif (Variables|Default|Getre)
        (if (<= (Variables|Default|Getframe) 1.0)
          (Variables|Default|Setframe 1.0)
          (if (not (Variables|Default|GetPause))
            (Sequencer|Player|Pause _geometrycache_2)
            (Variables|Default|SetPause true)
            (Variables|Default|Setplay false))
          (else
            (Variables|Default|Setframe (- (Variables|Default|Getframe) 1.0))))
        (else
          (Class|GeometryCacheComponent|PlayReversed _geometrycache)
          (Variables|Default|Setre true)
          (Variables|Default|SetPause false)
          (Variables|Default|Setplay false))))))

(event Input|KeyboardEvents|P
  (params (Key :type Key%20Structure :default "None"))
  (:Pressed
    (Variables|Default|Setstart_Origin true)
    (if true
      (Utilities|FlowControl|FlipFlop
        (:A
          (Variables|Default|Setlight true))
        (:B
          (Variables|Default|Setlight false))))))

(fn ConstructionScript)