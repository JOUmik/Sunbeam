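; Mushroom actor that plays a Geometry Cache animation forward and backward, toggled by the O key.
; Each press flips the Light state and plays or reverses a Timeline that scales the cache, with X and Y sharing one track.
; Tick holds the cache paused until the first press, then follows Light, counting ticks rather than elapsed time to pause playback at either end.
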(event EventBeginPlay)

(event EventTick
  (params (DeltaSeconds :type Float%20%28single-precision%29))
  (bind _geometrycache (Variables|Default|GetGeometryCache))
  (bind _geometrycache_2 (Variables|Default|GetGeometryCache))
  (if (not (Variables|Default|Getstart_Origin))
    (if (not (Variables|Default|GetPause))
      (Sequencer|Player|Pause _geometrycache_2)
      (Variables|Default|SetPause true))
    (elif (Variables|Default|Getlight)
      (if (Variables|Default|Getplay)
        (if (>= (Variables|Default|Getframe) 2.1e+02)
          (Variables|Default|Setframe 211.0)
          (if (not (Variables|Default|GetPause))
            (Sequencer|Player|Pause _geometrycache)
            (Variables|Default|SetPause true)
            (Variables|Default|Setre false))
          (else
            (Variables|Default|Setframe (+ (Variables|Default|Getframe) 1.0))))
        (else
          (Audio|Components|Audio|Play _geometrycache_2)
          (Variables|Default|Setplay true)
          (Variables|Default|SetPause false)
          (Variables|Default|Setre false)))
      (elif (Variables|Default|Getre)
        (if (<= (Variables|Default|Getframe) 1.0)
          (Variables|Default|Setframe 1.0)
          (if (not (Variables|Default|GetPause))
            (Sequencer|Player|Pause _geometrycache)
            (Variables|Default|SetPause true)
            (Variables|Default|Setplay false))
          (else
            (Variables|Default|Setframe (- (Variables|Default|Getframe) 1.0))))
        (else
          (Class|GeometryCacheComponent|PlayReversed _geometrycache_2)
          (Variables|Default|Setre true)
          (Variables|Default|SetPause false)
          (Variables|Default|Setplay false))))))

(event Input|KeyboardEvents|O
  (params (Key :type Key%20Structure :default "None"))
  (bind _geometrycache (Variables|Default|GetGeometryCache))
  (bind _returnvalue (Transformation|GetWorldTransform _geometrycache))
  (:Pressed
    (Variables|Default|Setstart_Origin true)
    (if true
      (Utilities|FlowControl|FlipFlop
        (:A
          (Variables|Default|Setlight true)
          (bind (_direction _newtrack_0 _newtrack_1 _newtrack_2) (Timeline|Timeline Play)
            (:Update
              (Transformation|SetWorldTransform _geometrycache (Math|Transform|MakeTransform (.location _returnvalue) (.rotation _returnvalue) (Math|Vector|MakeVector _newtrack_1 _newtrack_1 _newtrack_0)) false false))))
        (:B
          (Variables|Default|Setlight false)
          (Timeline|Timeline Reverse))))))

(fn ConstructionScript)