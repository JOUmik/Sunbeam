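; BP_Mashroom_New2 is a mushroom plant actor that toggles between grow and revert animations when the O key is pressed.
; It stores its root's world scale on BeginPlay, and a FlipFlop alternately plays and reverses a timeline.
; Each timeline update scales the root with separate width and height curves and feeds an alpha curve into the "Jianru" float on the NSMashroom1 Niagara effect.
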(event EventBeginPlay
  (Variables|Default|SetScale_0 (Transformation|GetWorldScale (Variables|Default|GetDefaultSceneRoot))))

(event EventTick
  (params (DeltaSeconds :type Float%20%28single-precision%29)))

(event Input|KeyboardEvents|O
  (params (Key :type Key%20Structure :default "None"))
  (bind _scale_0 (Variables|Default|GetScale_0))
  (bind (_x _y _z) (Math|Vector|BreakVector _scale_0))
  (:Pressed
    (Utilities|FlowControl|Sequence
      (:then_1
        (Utilities|FlowControl|FlipFlop
          (:A
            (bind (_direction _small_mashroom _small_mashroom_height _alpha) (Timeline|Timeline Play)
              (:Update
                (Transformation|SetWorldScale3D (Variables|Default|GetDefaultSceneRoot) (Math|Vector|MakeVector (* _small_mashroom _x) (* _small_mashroom _y) (* _small_mashroom_height _z)))
                (Niagara|SetNiagaraVariable(Float) (Variables|Default|GetNS_Mashroom1) "Jianru" _alpha))))
          (:B
            (Timeline|Timeline Reverse)))))))

(fn ConstructionScript)