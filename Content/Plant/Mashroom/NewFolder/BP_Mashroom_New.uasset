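; BP_Mashroom_New is an interactive mushroom plant that plays a growth-style animation forward when interaction ends and reverses it when interaction begins.
; A geometry cache and a shared Timeline run together, with the Timeline scaling the mesh from the scale cached at BeginPlay.
; The Timeline also toggles the Niagara effect, adjusts its height and drives its Ring and Jianru parameters.
; On finish, it pauses the cache and sets bloom status by direction.
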(event Custom|PlayInReverse
  (bind _geometrycache (Variables|Default|GetGeometryCache))
  (bind _ns_mashroom (Variables|Default|GetNS_Mashroom))
  (bind _niagara_location (Variables|Default|GetNiagara_Location))
  (bind (_x _y _z) (Math|Vector|BreakVector _niagara_location))
  (Utilities|FlowControl|Sequence
    (:then_0
      (Class|GeometryCacheComponent|PlayReversed _geometrycache)
      (Variables|Default|SetIsReversing true))
    (:then_1
      (bind (_direction _newtrack_0 _newtrack_2 _ring _lerp) (Timeline|Timeline Reverse)
        (:Update
          (Transformation|SetWorldScale3D _geometrycache (* _newtrack_0 (Variables|Default|GetScale)))
          (if (>= _newtrack_2 1.0)
            (Rendering|SetVisibility _ns_mashroom (>= _newtrack_2 1.0) false)
            (Transformation|SetWorldLocation _ns_mashroom (Math|Vector|MakeVector _x _y (* _newtrack_2 _z)) false false)
            (Niagara|SetNiagaraVariable(Float) _ns_mashroom "Ring" _ring)
            (Niagara|SetNiagaraVariable(Float) _ns_mashroom "Jianru" _lerp)
            (else
              (Rendering|SetVisibility _ns_mashroom (>= _newtrack_2 1.0) false))))
        (:Finished
          (Sequencer|Player|Pause _geometrycache)
          (Class|BeamFlowerBase|SetBloomStatus (not (Variables|Default|GetIsReversing))))))))

(event Custom|PlayFromBegin
  (bind _geometrycache (Variables|Default|GetGeometryCache))
  (bind _ns_mashroom (Variables|Default|GetNS_Mashroom))
  (bind _niagara_location (Variables|Default|GetNiagara_Location))
  (bind (_x _y _z) (Math|Vector|BreakVector _niagara_location))
  (Utilities|FlowControl|Sequence
    (:then_0
      (Audio|Components|Audio|Play _geometrycache)
      (Variables|Default|SetIsReversing false))
    (:then_1
      (bind (_direction _newtrack_0 _newtrack_2 _ring _lerp) (Timeline|Timeline Play)
        (:Update
          (Transformation|SetWorldScale3D _geometrycache (* _newtrack_0 (Variables|Default|GetScale)))
          (if (>= _newtrack_2 1.0)
            (Rendering|SetVisibility _ns_mashroom (>= _newtrack_2 1.0) false)
            (Transformation|SetWorldLocation _ns_mashroom (Math|Vector|MakeVector _x _y (* _newtrack_2 _z)) false false)
            (Niagara|SetNiagaraVariable(Float) _ns_mashroom "Ring" _ring)
            (Niagara|SetNiagaraVariable(Float) _ns_mashroom "Jianru" _lerp)
            (else
              (Rendering|SetVisibility _ns_mashroom (>= _newtrack_2 1.0) false))))
        (:Finished
          (Sequencer|Player|Pause _geometrycache)
          (Class|BeamFlowerBase|SetBloomStatus (not (Variables|Default|GetIsReversing))))))))

(event EventBeginPlay
  (if (Utilities|Operators|EqualEqual :A (Variables|Default|GetScale))
    (Variables|Default|SetScale (.scale (Transformation|GetWorldTransform (Variables|Default|GetGeometryCache))))
    (Variables|Default|SetNiagara_Location (Transformation|GetWorldLocation (Variables|Default|GetNS_Mashroom)))))

(event EventOnEndInteract
  (CallFunction|PlayfromBegin))

(event EventOnBeginInteract
  (params (BeamHitResult :type Hit%20Result%20Structure) (BeamLightSourceTag :type Gameplay%20Tag%20Structure))
  (CallFunction|PlayinReverse))

(event EventTick
  (params (DeltaSeconds :type Float%20%28single-precision%29)))

(event Input|KeyboardEvents|O
  (params (Key :type Key%20Structure :default "None")))

(fn ConstructionScript)