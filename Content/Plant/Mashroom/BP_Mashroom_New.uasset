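; Mushroom actor that toggles a geometry-cache animation and Niagara effect forward and backward with the O key.
; Two flip-flops reverse the cache playback and a timeline, which pauses the cache when finished.
; The timeline multiplies the mesh scale cached at BeginPlay, shows the effect once its track reaches 1, then drives the effect's height and "Ring" parameter.
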(event EventBeginPlay
  (if (Utilities|Operators|EqualEqual :A (Variables|Default|GetScale))
    (Variables|Default|SetScale (.scale (Transformation|GetWorldTransform (Variables|Default|GetGeometryCache))))
    (Variables|Default|SetNiagara_Location (Transformation|GetWorldLocation (Variables|Default|GetNS_Mashroom)))))

(event EventTick
  (params (DeltaSeconds :type Float%20%28single-precision%29)))

(event Input|KeyboardEvents|O
  (params (Key :type Key%20Structure :default "None"))
  (bind _geometrycache (Variables|Default|GetGeometryCache))
  (bind _ns_mashroom (Variables|Default|GetNS_Mashroom))
  (bind _niagara_location (Variables|Default|GetNiagara_Location))
  (bind (_x _y _z) (Math|Vector|BreakVector _niagara_location))
  (:Pressed
    (Utilities|FlowControl|Sequence
      (:then_0
        (Utilities|FlowControl|FlipFlop
          (:A
            (Audio|Components|Audio|Play _geometrycache))
          (:B
            (Class|GeometryCacheComponent|PlayReversed _geometrycache))))
      (:then_1
        (Utilities|FlowControl|FlipFlop
          (:A
            (bind (_direction _newtrack_0 _newtrack_2 _ring) (Timeline|Timeline Play)
              (:Update
                (Transformation|SetWorldScale3D _geometrycache (* _newtrack_0 (Variables|Default|GetScale)))
                (if (>= _newtrack_2 1.0)
                  (Rendering|SetVisibility _ns_mashroom (>= _newtrack_2 1.0) false)
                  (Transformation|SetWorldLocation _ns_mashroom (Math|Vector|MakeVector _x _y (* _newtrack_2 _z)) false false)
                  (Niagara|SetNiagaraVariable(Float) _ns_mashroom "Ring" _ring)
                  (else
                    (Rendering|SetVisibility _ns_mashroom (>= _newtrack_2 1.0) false))))
              (:Finished
                (Sequencer|Player|Pause _geometrycache))))
          (:B
            (Timeline|Timeline Reverse)))))))

(fn ConstructionScript)