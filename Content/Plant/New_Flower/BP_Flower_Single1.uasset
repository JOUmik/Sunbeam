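; Single flower actor that blooms and un-blooms through paired forward and reverse animation events.
; A Timeline drives geometry cache and static mesh scale from values captured at BeginPlay, plus the open and shine Niagara "Control" parameters, while the cache plays alongside.
; On finish it pauses the cache and sets bloom status, bursting particles after a forward bloom.
; Reversing a completed bloom restarts the close effect, fed the static mesh.
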(event EventBeginPlay
  (if (Utilities|Operators|EqualEqual :A (Variables|Default|GetScale))
    (Variables|Default|SetScale (.scale (Transformation|GetWorldTransform (Variables|Default|GetS_Butterfly_Weed_vkblbcdia_Var10_lod1))))
    (Variables|Default|SetFlower_Scale_0 (.scale (Transformation|GetWorldTransform (Variables|Default|GetGeometryCache))))
    (Class|NiagaraComponent|SetPaused (Variables|Default|GetNS_Flower_Open) true)
    (Class|NiagaraComponent|SetPaused (Variables|Default|GetNS_Flower_Close) true)
    (Class|NiagaraComponent|SetPaused (Variables|Default|GetNS_Flower_Shinning) true)
    (Class|NiagaraComponent|SetPaused (Variables|Default|GetNS_Flower_Burst) true)))

(event EventPlayBloomAnimForward
  (bind _geometrycache (Variables|Default|GetGeometryCache))
  (bind _s_butterfly_weed_vkblbcdia_var10_lod1 (Variables|Default|GetS_Butterfly_Weed_vkblbcdia_Var10_lod1))
  (bind _returnvalue (Transformation|GetWorldTransform _s_butterfly_weed_vkblbcdia_var10_lod1))
  (Utilities|FlowControl|Sequence
    (:then_0
      (Audio|Components|Audio|Play _geometrycache)
      (Variables|Default|SetIsReversing false)
      (Components|Activation|Activate (Variables|Default|GetNS_Flower_Open) false)
      (Components|Activation|Activate (Variables|Default|GetNS_Flower_Shinning) false))
    (:then_1
      (bind (_direction _newtrack_0 _newtrack_1 _newtrack_2 _niagara_switch _niagara_switch2) (Timeline|Timeline Play)
        (:Update
          (Transformation|SetWorldScale3D _geometrycache (* _newtrack_0 (Variables|Default|GetFlower_Scale_0)))
          (Transformation|SetWorldTransform _s_butterfly_weed_vkblbcdia_var10_lod1 (Math|Transform|MakeTransform (.location _returnvalue) (.rotation _returnvalue) (* (Math|Vector|MakeVector _newtrack_1 _newtrack_1 _newtrack_2) (Variables|Default|GetScale))) false false)
          (Niagara|SetNiagaraVariable(Float) (Variables|Default|GetNS_Flower_Open) "Control" _niagara_switch)
          (Niagara|SetNiagaraVariable(Float) (Variables|Default|GetNS_Flower_Shinning) "Control" _niagara_switch2))
        (:Finished
          (Sequencer|Player|Pause _geometrycache)
          (Class|BeamFlowerBase|SetBloomStatus (not (Variables|Default|GetIsReversing)))
          (if (not (Variables|Default|GetIsReversing))
            (Niagara|ResetSystem (Variables|Default|GetNS_Flower_Burst))
            (Variables|Default|SetDissolve true)
            (else
              (Variables|Default|SetDissolve false))))))))

(event EventPlayBloomAnimReverse
  (bind _geometrycache (Variables|Default|GetGeometryCache))
  (bind _ns_flower_close (Variables|Default|GetNS_Flower_Close))
  (bind _s_butterfly_weed_vkblbcdia_var10_lod1 (Variables|Default|GetS_Butterfly_Weed_vkblbcdia_Var10_lod1))
  (bind _returnvalue (Transformation|GetWorldTransform _s_butterfly_weed_vkblbcdia_var10_lod1))
  (Utilities|FlowControl|Sequence
    (:then_0
      (bind (_direction _newtrack_0 _newtrack_1 _newtrack_2 _niagara_switch _niagara_switch2) (Timeline|Timeline Reverse)
        (:Update
          (Transformation|SetWorldScale3D _geometrycache (* _newtrack_0 (Variables|Default|GetFlower_Scale_0)))
          (Transformation|SetWorldTransform _s_butterfly_weed_vkblbcdia_var10_lod1 (Math|Transform|MakeTransform (.location _returnvalue) (.rotation _returnvalue) (* (Math|Vector|MakeVector _newtrack_1 _newtrack_1 _newtrack_2) (Variables|Default|GetScale))) false false)
          (Niagara|SetNiagaraVariable(Float) (Variables|Default|GetNS_Flower_Open) "Control" _niagara_switch)
          (Niagara|SetNiagaraVariable(Float) (Variables|Default|GetNS_Flower_Shinning) "Control" _niagara_switch2))
        (:Finished
          (Sequencer|Player|Pause _geometrycache)
          (Class|BeamFlowerBase|SetBloomStatus (not (Variables|Default|GetIsReversing)))
          (if (not (Variables|Default|GetIsReversing))
            (Niagara|ResetSystem (Variables|Default|GetNS_Flower_Burst))
            (Variables|Default|SetDissolve true)
            (else
              (Variables|Default|SetDissolve false))))))
    (:then_1
      (Class|GeometryCacheComponent|PlayReversed _geometrycache)
      (Variables|Default|SetIsReversing true)
      (if (Variables|Default|GetDissolve)
        (Niagara|ResetSystem _ns_flower_close)
        (Class|NiagaraFunctionLibrary|OverrideSystemUserVariableStaticMeshComponent _ns_flower_close "Flower" _s_butterfly_weed_vkblbcdia_var10_lod1)))))

(fn ConstructionScript)