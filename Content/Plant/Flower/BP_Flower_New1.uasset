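; Flower actor that animates six geometry caches and a butterfly weed mesh when P is pressed.
; BeginPlay stores their original scales as baselines for timeline-driven scaling.
; The key loops over the caches through shared FlipFlops, alternating forward and reverse playback and timeline direction per element, with one timeline serving all iterations.
; Niagara positioning and direction logic is present but never runs.
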(event EventBeginPlay
  (if (Utilities|Operators|EqualEqual :A (Variables|Default|GetScale))
    (Variables|Default|SetScale (.scale (Transformation|GetWorldTransform (Variables|Default|GetS_Butterfly_Weed_vkblbcdia_Var10_lod1))))
    (bind _output_get (Variables|Default|SetVec_arr (Utilities|Array|MakeArray "0, 0, 0" "0, 0, 0" "0, 0, 0" "0, 0, 0" "0, 0, 0" "0, 0, 0")))
    (for (_array_element _array_index) (Utilities|Array|MakeArray (Variables|Default|GetGeometryCache) (Variables|Default|GetGeometryCache1) (Variables|Default|GetGeometryCache2) (Variables|Default|GetGeometryCache3) (Variables|Default|GetGeometryCache4) (Variables|Default|GetGeometryCache5))
      (Utilities|Array|SetArrayElem _output_get _array_index (.scale (Transformation|GetWorldTransform _array_element))))))

(event Input|KeyboardEvents|P
  (params (Key :type Key%20Structure :default "None"))
  (bind _s_butterfly_weed_vkblbcdia_var10_lod1 (Variables|Default|GetS_Butterfly_Weed_vkblbcdia_Var10_lod1))
  (bind _returnvalue (Transformation|GetWorldTransform _s_butterfly_weed_vkblbcdia_var10_lod1))
  (:Pressed
    (for (_array_element _array_index) (Utilities|Array|MakeArray (Variables|Default|GetGeometryCache) (Variables|Default|GetGeometryCache1) (Variables|Default|GetGeometryCache2) (Variables|Default|GetGeometryCache3) (Variables|Default|GetGeometryCache4) (Variables|Default|GetGeometryCache5))
      (Utilities|FlowControl|Sequence
        (:then_0
          (Utilities|FlowControl|FlipFlop
            (:A
              (Audio|Components|Audio|Play _array_element))
            (:B
              (Class|GeometryCacheComponent|PlayReversed _array_element))))
        (:then_1
          (Utilities|FlowControl|FlipFlop
            (:A
              (bind (_direction _newtrack_0 _newtrack_1 _newtrack_2) (Timeline|Timeline Play)
                (:Update
                  (Transformation|SetWorldScale3D _array_element (* _newtrack_0 (Utilities|Array|Get(acopy) (Variables|Default|GetVec_arr) _array_index)))
                  (Transformation|SetWorldTransform _s_butterfly_weed_vkblbcdia_var10_lod1 (Math|Transform|MakeTransform (.location _returnvalue) (.rotation _returnvalue) (* (Math|Vector|MakeVector _newtrack_1 _newtrack_1 _newtrack_2) (Variables|Default|GetScale))) false false))
                (:Finished
                  (Sequencer|Player|Pause _array_element))))
            (:B
              (Timeline|Timeline Reverse))))))))

(fn ConstructionScript)