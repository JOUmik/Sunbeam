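; Flower actor that blooms and un-blooms through forward and reverse animation events.
; On BeginPlay it caches the base scales of the weed mesh and six geometry cache flowers, if the stored plant scale is zero.
; The events play the caches forward or backward alongside a timeline that multiplies those base scales, stretching the weed mesh separately in Z.
; When the timeline finishes, it pauses the caches and sets bloom status from the direction.
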(event EventBeginPlay
  (if (Utilities|Operators|EqualEqual :A (Variables|Default|GetScale))
    (Variables|Default|SetScale (.scale (Transformation|GetWorldTransform (Variables|Default|GetS_Butterfly_Weed_vkblbcdia_Var10_lod1))))
    (Variables|Default|SetFlower_Scale_0 (.scale (Transformation|GetWorldTransform (Variables|Default|GetGeometryCache))))
    (Variables|Default|SetFlower_Scale_1 (.scale (Transformation|GetWorldTransform (Variables|Default|GetGeometryCache1))))
    (Variables|Default|SetFlower_Scale_2 (.scale (Transformation|GetWorldTransform (Variables|Default|GetGeometryCache2))))
    (Variables|Default|SetFlower_Scale_3 (.scale (Transformation|GetWorldTransform (Variables|Default|GetGeometryCache3))))
    (Variables|Default|SetFlower_Scale_4 (.scale (Transformation|GetWorldTransform (Variables|Default|GetGeometryCache4))))
    (Variables|Default|SetFlower_Scale_5 (.scale (Transformation|GetWorldTransform (Variables|Default|GetGeometryCache5))))))

(event EventPlayBloomAnimForward
  (bind _geometrycache (Variables|Default|GetGeometryCache))
  (bind _s_butterfly_weed_vkblbcdia_var10_lod1 (Variables|Default|GetS_Butterfly_Weed_vkblbcdia_Var10_lod1))
  (bind _returnvalue (Transformation|GetWorldTransform _s_butterfly_weed_vkblbcdia_var10_lod1))
  (Utilities|FlowControl|Sequence
    (:then_0
      (Audio|Components|Audio|Play _geometrycache)
      (Variables|Default|SetIsReversing false))
    (:then_1
      (bind (_direction _newtrack_0 _newtrack_1 _newtrack_2) (Timeline|Timeline Play)
        (:Update
          (Transformation|SetWorldScale3D _geometrycache (* _newtrack_0 (Variables|Default|GetFlower_Scale_0)))
          (Transformation|SetWorldScale3D (Variables|Default|GetGeometryCache1) (* _newtrack_0 (Variables|Default|GetFlower_Scale_1)))
          (Transformation|SetWorldScale3D (Variables|Default|GetGeometryCache2) (* _newtrack_0 (Variables|Default|GetFlower_Scale_2)))
          (Transformation|SetWorldScale3D (Variables|Default|GetGeometryCache3) (* _newtrack_0 (Variables|Default|GetFlower_Scale_3)))
          (Transformation|SetWorldScale3D (Variables|Default|GetGeometryCache4) (* _newtrack_0 (Variables|Default|GetFlower_Scale_4)))
          (Transformation|SetWorldScale3D (Variables|Default|GetGeometryCache5) (* _newtrack_0 (Variables|Default|GetFlower_Scale_5)))
          (Transformation|SetWorldTransform _s_butterfly_weed_vkblbcdia_var10_lod1 (Math|Transform|MakeTransform (.location _returnvalue) (.rotation _returnvalue) (* (Math|Vector|MakeVector _newtrack_1 _newtrack_1 _newtrack_2) (Variables|Default|GetScale))) false false))
        (:Finished
          (Sequencer|Player|Pause _geometrycache)
          (Class|BeamFlowerBase|SetBloomStatus (not (Variables|Default|GetIsReversing))))))))

(event EventPlayBloomAnimReverse
  (bind _geometrycache (Variables|Default|GetGeometryCache))
  (bind _s_butterfly_weed_vkblbcdia_var10_lod1 (Variables|Default|GetS_Butterfly_Weed_vkblbcdia_Var10_lod1))
  (bind _returnvalue (Transformation|GetWorldTransform _s_butterfly_weed_vkblbcdia_var10_lod1))
  (Utilities|FlowControl|Sequence
    (:then_0
      (Class|GeometryCacheComponent|PlayReversed _geometrycache)
      (Variables|Default|SetIsReversing true))
    (:then_1
      (bind (_direction _newtrack_0 _newtrack_1 _newtrack_2) (Timeline|Timeline Reverse)
        (:Update
          (Transformation|SetWorldScale3D _geometrycache (* _newtrack_0 (Variables|Default|GetFlower_Scale_0)))
          (Transformation|SetWorldScale3D (Variables|Default|GetGeometryCache1) (* _newtrack_0 (Variables|Default|GetFlower_Scale_1)))
          (Transformation|SetWorldScale3D (Variables|Default|GetGeometryCache2) (* _newtrack_0 (Variables|Default|GetFlower_Scale_2)))
          (Transformation|SetWorldScale3D (Variables|Default|GetGeometryCache3) (* _newtrack_0 (Variables|Default|GetFlower_Scale_3)))
          (Transformation|SetWorldScale3D (Variables|Default|GetGeometryCache4) (* _newtrack_0 (Variables|Default|GetFlower_Scale_4)))
          (Transformation|SetWorldScale3D (Variables|Default|GetGeometryCache5) (* _newtrack_0 (Variables|Default|GetFlower_Scale_5)))
          (Transformation|SetWorldTransform _s_butterfly_weed_vkblbcdia_var10_lod1 (Math|Transform|MakeTransform (.location _returnvalue) (.rotation _returnvalue) (* (Math|Vector|MakeVector _newtrack_1 _newtrack_1 _newtrack_2) (Variables|Default|GetScale))) false false))
        (:Finished
          (Sequencer|Player|Pause _geometrycache)
          (Class|BeamFlowerBase|SetBloomStatus (not (Variables|Default|GetIsReversing))))))))

(fn ConstructionScript)