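; BP_LampBase is a lamp plant base that plays its bloom and close visual effects through several Niagara systems.
; A Timeline runs forward or in reverse, driving the Control parameter on the open and shining effects.
; A finished bloom fires a burst, sets Dissolve and activates the main Niagara, whose radius comes from the glow sphere.
; Reversing resets the close effect if dissolved, then deactivates the main system when the Timeline finishes.
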(event EventPlayBloomAnimForward
  (Variables|Default|SetIsReversing false)
  (Utilities|FlowControl|Sequence
    (:then_0
      ;[1 1 1] Active_open
      (Components|Activation|Activate (Variables|Default|GetNiagara_Shining) false)
      (Components|Activation|Activate (Variables|Default|GetNiagara_Open) false))
    (:then_1
      (bind (_direction _newtrack_0 _newtrack_1 _newtrack_2 _niagara_switch _niagara_switch2) (Timeline|Timeline Play)
        (:Update
          ;[1 1 1] Set alpha control
          (Niagara|SetNiagaraVariable(Float) (Variables|Default|GetNiagara_Open) "Control" _niagara_switch)
          (Niagara|SetNiagaraVariable(Float) (Variables|Default|GetNiagara_Shining) "Control" _niagara_switch2))
        (:Finished
          (Class|BeamFlowerBase|SetBloomStatus (not (Variables|Default|GetIsReversing)))
          ;[1 1 1] Finish_Burst
          (if (not (Variables|Default|GetIsReversing))
            (Niagara|ResetSystem (Variables|Default|GetNiagara_Burst))
            (Variables|Default|SetDissolve true)
            (Components|Activation|Activate (Variables|Default|GetNiagara) false)
            (else
              (Variables|Default|SetDissolve false)
              (Components|Activation|Deactivate (Variables|Default|GetNiagara)))))))))

(event EventPlayBloomAnimReverse
  (Variables|Default|SetIsReversing true)
  (Utilities|FlowControl|Sequence
    (:then_0
      ;[1 1 1] Close_Effect
      (if (Variables|Default|GetDissolve)
        (Niagara|ResetSystem (Variables|Default|GetNiagara_Close))
        (Class|NiagaraFunctionLibrary|OverrideSystemUserVariableStaticMeshComponent 0 "Flower")))
    (:then_1
      (bind (_direction _newtrack_0 _newtrack_1 _newtrack_2 _niagara_switch _niagara_switch2) (Timeline|Timeline Reverse)
        (:Update
          ;[1 1 1] Set alpha control
          (Niagara|SetNiagaraVariable(Float) (Variables|Default|GetNiagara_Open) "Control" _niagara_switch)
          (Niagara|SetNiagaraVariable(Float) (Variables|Default|GetNiagara_Shining) "Control" _niagara_switch2))
        (:Finished
          (Class|BeamFlowerBase|SetBloomStatus (not (Variables|Default|GetIsReversing)))
          ;[1 1 1] Finish_Burst
          (if (not (Variables|Default|GetIsReversing))
            (Niagara|ResetSystem (Variables|Default|GetNiagara_Burst))
            (Variables|Default|SetDissolve true)
            (Components|Activation|Activate (Variables|Default|GetNiagara) false)
            (else
              (Variables|Default|SetDissolve false)
              (Components|Activation|Deactivate (Variables|Default|GetNiagara)))))))))

(event EventBeginPlay
  (Class|NiagaraComponent|SetPaused (Variables|Default|GetNiagara_Open) true)
  (Class|NiagaraComponent|SetPaused (Variables|Default|GetNiagara_Close) true)
  (Class|NiagaraComponent|SetPaused (Variables|Default|GetNiagara_Shining) true)
  (Class|NiagaraComponent|SetPaused (Variables|Default|GetNiagara_Burst) true)
  (Class|NiagaraComponent|SetPaused (Variables|Default|GetNiagara) true)
  (Niagara|SetNiagaraVariable(Float) (Variables|Default|GetNiagara) "User_Radius" (Variables|/Script/Engine.SphereComponent|GetSphereRadius (Variables|Default|GetGlowingRadiusComponent))))

(fn ConstructionScript)