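; Test actor that runs three cube meshes along a spline like linked train cars.
; The I key flip-flops a switch that starts and stops the motion.
; While on, Tick places each cube at the spline's world transform, offset by index times TrainLength, with a fixed scale.
; Distance advances by Speed times delta time inside the loop, so it grows once per cube each frame.
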(event EventBeginPlay)

(event Collision|EventActorBeginOverlap
  (params (OtherActor :type Actor%20Object%20Reference)))

(event EventTick
  (params (DeltaSeconds :type Float%20%28single-precision%29))
  (if (Variables|Default|GetSwitch)
    (for (_array_element _array_index) (Utilities|Array|MakeArray (Variables|Default|GetCube) (Variables|Default|GetCube1) (Variables|Default|GetCube2))
      (bind _output_get (Variables|Default|SetDistance (+ (* DeltaSeconds (Variables|Default|GetSpeed)) (Variables|Default|GetDistance))))
      (Transformation|SetWorldTransform _array_element (Math|Transform|MakeTransform (.location (Spline|GetTransformatDistanceAlongSpline (Variables|Default|GetSpline) (+ _output_get (* _array_index (Variables|Default|GetTrain_Length))) "World" false)) (.rotation (Spline|GetTransformatDistanceAlongSpline (Variables|Default|GetSpline) (+ _output_get (* _array_index (Variables|Default|GetTrain_Length))) "World" false)) "1.000000,0.500000,0.500000") false false))))

(event Input|KeyboardEvents|I
  (params (Key :type Key%20Structure :default "None"))
  (:Pressed
    (Utilities|FlowControl|FlipFlop
      (:A
        (Variables|Default|SetSwitch true))
      (:B
        (Variables|Default|SetSwitch false)))))

(fn ConstructionScript)